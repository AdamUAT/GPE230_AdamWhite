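; MazeGameInstance is the game instance that loads or creates the maze game's save data on startup.
; On Init it checks for an existing save slot and loads it as a MazeSaveGame into SaveData.
; If none exists, it creates a new save with master, music and SFX volumes at full, stores it in SaveData and writes it to the slot.
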(event `self.ReceiveInit`
  (bind _returnvalue (`GameplayStatics.DoesSaveGameExist` (`self.SaveSlotName`)))
  (if _returnvalue
    (bind _returnvalue_2 (`GameplayStatics.LoadGameFromSlot` (`self.SaveSlotName`)))
    (bind _asmaze_save_game (cast `MazeSaveGame` _returnvalue_2))
    (set `self.saveData` _asmaze_save_game)
    (else
      (bind _returnvalue_3 (`GameplayStatics.CreateSaveGameObject` "/Script/GPE230_AdamWhite.MazeSaveGame"))
      (set `MazeSaveGame.masterVolumeSetting` 1.0 _returnvalue_3)
      (set `MazeSaveGame.musicVolumeSetting` 1.0 _returnvalue_3)
      (set `MazeSaveGame.sfxVolumeSetting` 1.0 _returnvalue_3)
      (bind _output_get (set `self.saveData` _returnvalue_3))
      (`GameplayStatics.SaveGameToSlot` _output_get (`self.SaveSlotName`)))))