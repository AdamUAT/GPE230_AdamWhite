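; EnemyStunnable is a component Blueprint that temporarily stuns its owning NPCEnemyBP.
; The Stunned event sets the stun flag, waits for StunDuration, then clears it.
; SetIsStunned writes that flag to the IsStunned key on the AI controller's blackboard, doing nothing if the owner is not an NPCEnemyBP.
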(event `self.Stunned`
  (`self.SetIsStunned` true)
  (`KismetSystemLibrary.Delay` (`self.StunDuration`))
  (`self.SetIsStunned` false))

(fn `SetIsStunned`
  (params (IsStunned :type Boolean))
  (bind _asnpcenemy_bp (cast `/Game/AdamUAT/Blueprints/NPCEnemyBP` (`self.GetOwner`)))
  (`BlackboardComponent.SetValueAsBool` (`AIBlueprintHelperLibrary.GetBlackboard` (`Pawn.GetController` _asnpcenemy_bp)) "IsStunned" IsStunned))