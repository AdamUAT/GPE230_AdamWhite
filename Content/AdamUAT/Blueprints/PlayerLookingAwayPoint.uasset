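; PlayerLookingAwayPoint is a placeable point that reports whether it sits outside the player's view.
; IsNotVisible compares camera yaw with the look-at yaw to the point, requiring it to fall outside half the FOV plus a margin and not be too close to the camera.
; The test ignores pitch and occlusion, and the yaw difference is not normalized for angle wraparound.
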(event `self.ReceiveTick`
  (params (DeltaSeconds :type "Float (single-precision)")))

(fn `IsNotVisible`
  (returns (Result :type Boolean))
  (bind _returnvalue (`GameplayStatics.GetPlayerCameraManager` 0))
  (bind _returnvalue_2 (`self.K2_GetActorLocation`))
  (bind _returnvalue_3 (`PlayerCameraManager.GetCameraLocation` _returnvalue))
  (bind (_returnvalue_roll _returnvalue_pitch _returnvalue_yaw) (`KismetMathLibrary.BreakRotator` (`PlayerCameraManager.GetCameraRotation` _returnvalue)))
  (bind (_returnvalue_roll_2 _returnvalue_pitch_2 _returnvalue_yaw_2) (`KismetMathLibrary.BreakRotator` (`KismetMathLibrary.FindLookAtRotation` _returnvalue_3 _returnvalue_2)))
  (bind _returnvalue_4 (/ (`PlayerCameraManager.GetFOVAngle` _returnvalue) 2.0))
  (return (and (not (`KismetMathLibrary.InRange_FloatFloat` (- _returnvalue_yaw _returnvalue_yaw_2) (- 0.0 15.0 _returnvalue_4) (+ 0.0 15.0 _returnvalue_4) false false)) (>= (`KismetMathLibrary.Vector_Distance` _returnvalue_3 _returnvalue_2) 100.0))))

(fn `UserConstructionScript`)