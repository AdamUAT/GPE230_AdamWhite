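; WinDetector is a pickup Blueprint that completes a maze level and triggers the victory screen when collected.
; On pickup, it raises the furthest completed level in the MazeGameInstance save data to a hard-coded 3 if lower, then saves to the slot.
; It then casts the player to MazeCharacterBP and opens the victory screen through its MazePlayerController.
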(event `self.OnPickup`
  (params (player :type "Actor Object Reference"))
  (bind _asmaze_game_instance (cast `/Game/AdamUAT/Blueprints/MazeGameInstance` (`GameplayStatics.GetGameInstance`)))
  (bind _savedata (`/Game/AdamUAT/Blueprints/MazeGameInstance.saveData` _asmaze_game_instance))
  (if (not (> (`MazeSaveGame.furthestCompletedLevel` _savedata) 2))
    (set `MazeSaveGame.furthestCompletedLevel` 3 _savedata)
    (`GameplayStatics.SaveGameToSlot` _savedata (`/Game/AdamUAT/Blueprints/MazeGameInstance.SaveSlotName` _asmaze_game_instance)))
  (bind _asmaze_character_bp (cast `/Game/AdamUAT/Blueprints/MazeCharacterBP` player))
  (bind _asmaze_player_controller (cast `MazePlayerController` (`Pawn.GetController` _asmaze_character_bp)))
  (`MazePlayerController.OpenVictoryScreen` _asmaze_player_controller))

(fn `UserConstructionScript`
  (`parent.UserConstructionScript`))