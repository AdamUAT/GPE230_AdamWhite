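; HealthPickup is a pickup Blueprint that restores health to the maze character that collects it.
; Its OnPickup event casts the player to MazeCharacterBP, calls Heal on that character's Health with HealthAmount, then destroys the pickup.
; If the cast fails, nothing happens and the pickup stays; BeginPlay, overlap and Tick are disabled stubs.
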(event `self.OnPickup`
  (params (player :type "Actor Object Reference"))
  (bind _asmaze_character_bp (cast `/Game/AdamUAT/Blueprints/MazeCharacterBP` player))
  (`Health.Heal` (`/Game/AdamUAT/Blueprints/MazeCharacterBP.Health` _asmaze_character_bp) (`self.HealthAmount`))
  (`self.K2_DestroyActor`))

(fn `UserConstructionScript`
  (`parent.UserConstructionScript`))