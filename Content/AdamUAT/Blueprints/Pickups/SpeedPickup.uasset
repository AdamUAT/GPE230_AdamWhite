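; Speed pickup that temporarily boosts the walk speed and acceleration of the MazeCharacterBP that collects it.
; On pickup it scales both through ApplyBoost by the SpeedBoost percentage, then hides itself and disables its collision.
; After Duration it calls ApplyBoost with the inverse percentage, -b/(b+1), to undo the boost without caching original values, then destroys itself.
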(event `self.OnPickup`
  (params (player :type "Actor Object Reference"))
  (bind _returnvalue (/ (`self.SpeedBoost`) 100.0))
  (bind _asmaze_character_bp (cast `/Game/AdamUAT/Blueprints/MazeCharacterBP` player))
  (bind _charactermovement (`Character.CharacterMovement` _asmaze_character_bp))
  (`self.ApplyBoost` (/ (`self.SpeedBoost`) 100.0) _charactermovement)
  (`PrimitiveComponent.SetCollisionEnabled` (`self.CollisionComponent`) "NoCollision")
  (`self.SetActorHiddenInGame` true)
  (`KismetSystemLibrary.Delay` (`self.Duration`))
  (`self.ApplyBoost` (/ _returnvalue (+ _returnvalue 1.0) -1.0) _charactermovement)
  (`self.K2_DestroyActor`))

(fn `ApplyBoost`
  (params (Amount :type "Float (double-precision)") (MovementComp :type "CharacterMovementComponent Object Reference"))
  (bind _returnvalue (`CharacterMovementComponent.GetMaxAcceleration` MovementComp))
  (bind _returnvalue_2 (`MovementComponent.GetMaxSpeed` MovementComp))
  (`|ExecutionSequence`
    (:`then_0`
      (set `CharacterMovementComponent.MaxWalkSpeed` (+ _returnvalue_2 (* _returnvalue_2 Amount)) MovementComp))
    (:`then_1`
      (set `CharacterMovementComponent.MaxAcceleration` (+ _returnvalue (* _returnvalue Amount)) MovementComp))))

(fn `UserConstructionScript`
  (`parent.UserConstructionScript`))